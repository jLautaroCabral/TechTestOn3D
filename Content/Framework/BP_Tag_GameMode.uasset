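; Game mode for the Tag game that gathers connecting players and starts the level once all have arrived.
; It collects tag player controllers until the count matches the game instance's connected-player number, then respawns each at the PlayerStart named by its index.
; After a short delay it triggers each controller's start countdown, then enables all input when the countdown ends.
; Logouts remove the controller and lower the expected count.
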(event Custom|LevelStart
  (Utilities|FlowControl|Delay 0.2)
  (for _array_element (Variables|Default|GetAll_ConnectedControllers)
    (Default|GameStartCountdown _array_element))
  (Utilities|FlowControl|Delay 3.0)
  (for _array_element_2 (Variables|Default|GetAll_ConnectedControllers)
    (Default|EnableAllInput _array_element_2)))

(event EventHandleStartingNewPlayer
  (params (NewPlayer :type Player%20Controller%20Object%20Reference))
  (bind _asbp_tag_player_controller (Utilities|Casting|CastToBP_TagPlayerController NewPlayer))
  (Utilities|Array|Add (Variables|Default|GetAll_ConnectedControllers) _asbp_tag_player_controller)
  (bind _asbp_tag_game_instance (Utilities|Casting|CastToBP_Tag_GameInstance (Game|GetGameInstance)))
  (Variables|Default|SetNum%20Expected%20%20Players (Variables|/Game/Framework/BP_Tag_GameInstance.BP_Tag_GameInstance_C|GetNum%20Connected%20Players _asbp_tag_game_instance))
  (if (== (Utilities|Array|Length (Variables|Default|GetAll_ConnectedControllers)) (Variables|Default|GetNum%20Expected%20%20Players))
    (Utilities|FlowControl|Delay 0.5)
    (for (_array_element _array_index) (Variables|Default|GetAll_ConnectedControllers)
      (Class|GameModeBase|RestartPlayeratPlayerStart _array_element (Class|GameModeBase|FindPlayerStart _array_element (Utilities|String|ToString(Integer) _array_index))))
    (CallFunction|LevelStart)))

(event EventOnLogout
  (params (ExitingController :type Controller%20Object%20Reference))
  (bind _asbp_tag_player_controller (Utilities|Casting|CastToBP_TagPlayerController ExitingController))
  (Utilities|Array|RemoveItem (Variables|Default|GetAll_ConnectedControllers) _asbp_tag_player_controller)
  (Math|Integer|DecrementInt (Variables|Default|GetNum%20Expected%20%20Players)))

(fn ConstructionScript)