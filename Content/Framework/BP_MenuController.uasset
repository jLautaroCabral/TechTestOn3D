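; Player controller for the main menu and multiplayer lobby that manages lobby and loading screen widgets, UI-only input and leaving a session.
; Initial setup loads or creates the saved player profile, then passes it through Server_UpdateLobby, which has BP_MainMenu_GameMode update the lobby.
; UpdatePlayerNames refreshes the lobby widget's name list from supplied profiles.
; Ending a client session destroys it and opens the main menu map.
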(event Custom|EndClientSession
  (|DestroySession self
    (:then
      (Game|OpenLevel(byName) "MainMenu_Map"))))

(event Custom|CreateLobbbyMenu
  (CallFunction|UIShowLobbyMenu))

(event Custom|Initial_Setup
  (CallFunction|LoadSavedProfile)
  (CallFunction|ServerUpdateLobby (Variables|Default|GetPlayer_Profile_Info)))

(event Custom|UpdatePlayerNames
  (params (Player_Profiles :type Array%20of%20S%20Player%20Profile%20Structures))
  (bind _wp_lobbymenu (Variables|Default|GetWP_LobbyMenu))
  (Utilities|IsValid _wp_lobbymenu
    (:Is%20Valid
      (Default|ClearPlayerNames _wp_lobbymenu)
      (Default|UpdatePlayerNames _wp_lobbymenu Player_Profiles))))

(event Custom|Server_UpdateLobby
  (params (Player_Profile :type S%20Player%20Profile%20Structure))
  (Variables|Default|SetPlayer_Profile_Info Player_Profile)
  (bind _asbp_main_menu_game_mode (Utilities|Casting|CastToBP_MainMenu_GameMode (Game|GetGameMode)))
  (Default|UpdateLobby _asbp_main_menu_game_mode true))

(event Custom|CreateLoadScreen
  (CallFunction|UIShowLoadScreen))

(event EventBeginPlay
  (if (Pawn|IsLocalController)
    (Variables|Default|SetbShowMouseCursor false)
    (Input|SetInputModeUIOnly self 0 "DoNotLock" false)))

(fn ConstructionScript)

(fn UIShowLoadScreen
  (Viewport|RemoveAllWidgets)
  (Utilities|IsValid (Variables|Default|GetWP_LoadScreen)
    (:Is%20Valid
      _)
    (:Is%20Not%20Valid
      (bind _returnvalue (UserInterface|CreateWidget "/Game/Widgets/WP_LoadingScreen.WP_LoadingScreen_C" self))
      (Variables|Default|SetWP_LoadScreen _returnvalue)))
  (UserInterface|Viewport|AddtoViewport (Variables|Default|GetWP_LoadScreen) 0)
  (return))

(fn UIShowLobbyMenu
  (Utilities|IsValid (Variables|Default|GetWP_LobbyMenu)
    (:Is%20Valid
      _)
    (:Is%20Not%20Valid
      (bind _returnvalue (UserInterface|CreateWidget "/Game/Widgets/WP_LobbyMenu.WP_LobbyMenu_C" self))
      (Variables|Default|SetWP_LobbyMenu _returnvalue)))
  (UserInterface|Viewport|AddtoViewport (Variables|Default|GetWP_LobbyMenu) 0)
  (return))

(fn LoadSavedProfile
  (bind _returnvalue (SaveGame|DoesSaveGameExist (Variables|Default|GetPlayer_Profile_Slot)))
  (if _returnvalue
    _
    (else
      (bind _returnvalue_2 (SaveGame|CreateSaveGameObject "/Game/SavedGame/SG_PlayerProfile.SG_PlayerProfile_C"))
      (SaveGame|SaveGametoSlot _returnvalue_2 (Variables|Default|GetPlayer_Profile_Slot))))
  (bind _returnvalue_3 (SaveGame|LoadGamefromSlot (Variables|Default|GetPlayer_Profile_Slot)))
  (bind _assg_player_profile (Utilities|Casting|CastToSG_PlayerProfile _returnvalue_3))
  (Variables|Default|SetPlayer_Profile_Info (Variables|/Game/SavedGame/SG_PlayerProfile.SG_PlayerProfile_C|GetPlayerProfile _assg_player_profile)))