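; Game instance for a multiplayer Tag game that manages menus, the player profile and session travel.
; It creates and caches main, multiplayer and pause widgets, with the pause toggle switching input mode and HUD without calling SetGamePaused.
; The player name persists through an SG_PlayerProfile save slot, checked when the main menu opens.
; It hosts LAN sessions into a listen-server lobby, joins found sessions and changes maps via servertravel.
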(event Custom|Change_PlayerName
  (params (PlayerName :type Text))
  (Variables|Default|SetPlayer_Profile_Info (Utilities|Struct|MakeS_PlayerProfile PlayerName))
  (CallFunction|SaveProfile))

(event Custom|CreateMPSession
  (|Session (Game|GetPlayerController 0) 4 true
    (:OnSuccess
      (Game|OpenLevel(byName) "LobbyMenu_Map" true "listen"))))

(event Custom|JoinMPSession
  (params (SessionResult :type Blueprint%20Session%20Result%20Structure))
  (|JoinSession (Game|GetPlayerController 0) SessionResult))

(event Custom|TravelToMap
  (params (NumConnectedPlayers :type Integer) (MapName :type String))
  (Variables|Default|SetNum%20Connected%20Players NumConnectedPlayers)
  (Development|ExecuteConsoleCommand (Utilities|String|Append "servertravel " MapName) (Game|GetPlayerController 0)))

(fn UIShowMultiplayerMenu
  (Utilities|IsValid (Variables|Default|GetWP_MultiplayerMenu)
    (:Is%20Valid
      _)
    (:Is%20Not%20Valid
      (bind _returnvalue (UserInterface|CreateWidget "/Game/Widgets/WP_MultiplayerMenu.WP_MultiplayerMenu_C" (Game|GetPlayerController 0)))
      (Variables|Default|SetWP_MultiplayerMenu _returnvalue)))
  (UserInterface|Viewport|AddtoViewport (Variables|Default|GetWP_MultiplayerMenu) 0))

(fn UIShowMainMenu
  (bind _returnvalue (Game|GetPlayerController 0))
  (Utilities|IsValid (Variables|Default|GetWP_MainMenu)
    (:Is%20Valid
      _)
    (:Is%20Not%20Valid
      (bind _returnvalue_2 (UserInterface|CreateWidget "/Game/Widgets/WP_MainMenu.WP_MainMenu_C" _returnvalue))
      (Variables|Default|SetWP_MainMenu _returnvalue_2)))
  (UserInterface|Viewport|AddtoViewport (Variables|Default|GetWP_MainMenu) 0)
  (Input|SetInputModeUIOnly _returnvalue 0 "DoNotLock" false)
  (Variables|/Script/Engine.PlayerController|SetbShowMouseCursor _returnvalue true)
  (CallFunction|CheckforSavedProfile)
  (Rendering|Components|TextRender|SetText (Variables|/Game/Widgets/WP_MainMenu.WP_MainMenu_C|GetInput_PlayerName (Variables|Default|GetWP_MainMenu)) (Utilities|Struct|BreakS_PlayerProfile (Variables|Default|GetPlayer_Profile_Info)))
  (return))

(fn CheckforSavedProfile
  (bind _returnvalue (SaveGame|DoesSaveGameExist (Variables|Default|GetPlayerProfile_Slot)))
  (if _returnvalue
    (bind _assg_player_profile (CallFunction|LoadProfile))
    (Variables|Default|SetSG_Player_Profile _assg_player_profile)
    (else
      (CallFunction|SaveProfile)))
  (return))

(fn LoadProfile
  (bind _returnvalue (SaveGame|LoadGamefromSlot (Variables|Default|GetPlayerProfile_Slot)))
  (bind _assg_player_profile (Utilities|Casting|CastToSG_PlayerProfile _returnvalue))
  (Variables|Default|SetPlayer_Profile_Info (Variables|/Game/SavedGame/SG_PlayerProfile.SG_PlayerProfile_C|GetPlayerProfile _assg_player_profile))
  (return _assg_player_profile))

(fn SaveProfile
  (Utilities|IsValid (Variables|Default|GetSG_Player_Profile)
    (:Is%20Valid
      _)
    (:Is%20Not%20Valid
      (bind _returnvalue (SaveGame|CreateSaveGameObject "/Game/SavedGame/SG_PlayerProfile.SG_PlayerProfile_C"))
      (Variables|Default|SetSG_Player_Profile _returnvalue)))
  (Variables|/Game/SavedGame/SG_PlayerProfile.SG_PlayerProfile_C|SetPlayerProfile (Variables|Default|GetSG_Player_Profile) (Variables|Default|GetPlayer_Profile_Info))
  (SaveGame|SaveGametoSlot (Variables|Default|GetSG_Player_Profile) (Variables|Default|GetPlayerProfile_Slot))
  (return))

(fn UIShowPauseMenu
  (bind _returnvalue (Game|GetPlayerController 0))
  (Utilities|IsValid (Variables|Default|GetWP_PauseMenu)
    (:Is%20Valid
      _)
    (:Is%20Not%20Valid
      (bind _returnvalue_2 (UserInterface|CreateWidget "/Game/Widgets/WP_PauseMenu.WP_PauseMenu_C" _returnvalue))
      (Variables|Default|SetWP_PauseMenu _returnvalue_2)))
  (UserInterface|Viewport|AddtoViewport (Variables|Default|GetWP_PauseMenu) 0)
  (Input|SetInputModeUIOnly _returnvalue 0 "DoNotLock" false)
  (Variables|/Script/Engine.PlayerController|SetbShowMouseCursor _returnvalue true))

(fn TogglePauseGame
  (bind _returnvalue (Game|GetPlayerController 0))
  (if (Variables|Default|GetMP_IsPauseMenuVisible)
    (Variables|Default|SetMP_IsPauseMenuVisible false)
    (Widget|RemovefromParent (Variables|Default|GetWP_PauseMenu))
    (Input|SetInputModeGameOnly _returnvalue false)
    (Variables|/Script/Engine.PlayerController|SetbShowMouseCursor _returnvalue false)
    (bind _asbp_tag_player_controller (Utilities|Casting|CastToBP_TagPlayerController _returnvalue))
    (Default|UnHideinGameHUD _asbp_tag_player_controller)
    (else
      (Variables|Default|SetMP_IsPauseMenuVisible true)
      (LocalVariables|SetLcl_IsGamePaused true)
      (CallFunction|UIShowPauseMenu)))
  (return (LocalVariables|GetLcl_IsGamePaused)))